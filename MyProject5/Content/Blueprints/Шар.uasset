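; Шар (Ball) is a child Blueprint actor whose overlap response is gated by a Люк (Hatch) child actor.
; On overlap it casts that child actor to Люк and runs the parent's overlap logic only while the hatch's Free flag is true.
; Its Action function destroys the actor, then sets Free to true.
; The construction script simply defers to the parent.
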(event EventBeginPlay)

(event Collision|EventActorBeginOverlap
  (params (OtherActor :type Actor%20Object%20Reference))
  (bind _asлюк (Utilities|Casting|CastToЛюк (Variables|/Script/Engine.ChildActorComponent|GetChildActor (Variables|Default|GetЛюк))))
  (if (Variables|/Game/Blueprints/eventObj.eventObj_C|GetFree _asлюк)
    (|CallParentFunction OtherActor)))

(event EventTick
  (params (DeltaSeconds :type Float%20%28single-precision%29)))

(fn ConstructionScript
  (|CallParentFunction))

(fn Action
  (Actor|DestroyActor)
  (Variables|Default|SetFree true))