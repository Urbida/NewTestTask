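; Hatch (Люк) interactable held by four nut (Гайка) child actors, which becomes usable only once all four nuts are free.
; While an actor overlaps it, a 0.2-second Delay loop polls each nut's Free flag and forwards BeginOverlap to the parent class when all are set.
; End overlap stops the polling and calls the parent.
; Action marks the hatch Free and hides it along with its nuts.
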(event Collision|EventActorBeginOverlap
  (params (OtherActor :type Actor%20Object%20Reference))
  (Variables|Default|SetOver true)
  (if (Variables|Default|GetOver) :!label _label
    (bind _asгайка (Utilities|Casting|CastToГайка (Variables|/Script/Engine.ChildActorComponent|GetChildActor (Variables|Default|GetГайка))))
    (bind _asгайка_2 (Utilities|Casting|CastToГайка (Variables|/Script/Engine.ChildActorComponent|GetChildActor (Variables|Default|GetГайка1))))
    (bind _asгайка_3 (Utilities|Casting|CastToГайка (Variables|/Script/Engine.ChildActorComponent|GetChildActor (Variables|Default|GetГайка2))))
    (bind _asгайка_4 (Utilities|Casting|CastToГайка (Variables|/Script/Engine.ChildActorComponent|GetChildActor (Variables|Default|GetГайка3))))
    (if (Math|Boolean|ANDBoolean (Variables|/Game/Blueprints/eventObj.eventObj_C|GetFree _asгайка_4) (Variables|/Game/Blueprints/eventObj.eventObj_C|GetFree _asгайка_3) (Variables|/Game/Blueprints/eventObj.eventObj_C|GetFree _asгайка_2) (Variables|/Game/Blueprints/eventObj.eventObj_C|GetFree _asгайка))
      (|CallParentFunction OtherActor)
      (else
        (Utilities|FlowControl|Delay 0.2)
        (goto _label)))))

(event Collision|EventActorEndOverlap
  (params (OtherActor :type Actor%20Object%20Reference))
  (Variables|Default|SetOver false)
  (|CallParentFunction OtherActor))

(fn ConstructionScript
  (|CallParentFunction))

(fn Action
  (Variables|Default|SetFree true)
  (CallFunction|Hide)
  (bind _asгайка (Utilities|Casting|CastToГайка (Variables|/Script/Engine.ChildActorComponent|GetChildActor (Variables|Default|GetГайка))))
  (Default|Hide _asгайка)
  (bind _asгайка_2 (Utilities|Casting|CastToГайка (Variables|/Script/Engine.ChildActorComponent|GetChildActor (Variables|Default|GetГайка1))))
  (Default|Hide _asгайка_2)
  (bind _asгайка_3 (Utilities|Casting|CastToГайка (Variables|/Script/Engine.ChildActorComponent|GetChildActor (Variables|Default|GetГайка2))))
  (Default|Hide _asгайка_3)
  (bind _asгайка_4 (Utilities|Casting|CastToГайка (Variables|/Script/Engine.ChildActorComponent|GetChildActor (Variables|Default|GetГайка3))))
  (Default|Hide _asгайка_4))